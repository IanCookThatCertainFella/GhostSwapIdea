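; BP_Chest is an interactable chest that opens when the player enters its sphere and closes when they leave.
; A Timeline rotates the Hinge for both directions, driven by OpenChest's flag, where false opens and true closes.
; When opening finishes, it shows a W_ChestMenu created at BeginPlay from BPCInventory, shows the player's inventory and registers its own with GM_SaveLoad's LevelState.
; LoadInventory restores the component's EnumInventory.
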(event OnComponentBeginOverlap(Sphere)
  (params (OverlappedComponent :type Primitive%20Component%20Object%20Reference) (OtherActor :type Actor%20Object%20Reference) (OtherComp :type Primitive%20Component%20Object%20Reference) (OtherBodyIndex :type Integer) (bFromSweep :type Boolean) (SweepResult :type Hit%20Result%20Structure%20%28by%20ref%29))
  (bind _asbp_first_person_swap (Utilities|Casting|CastToBP_FirstPersonSwap OtherActor))
  (if (Actor|ActorHasTag OtherActor "Player")
    (Development|PrintText (Utilities|Text|FormatText "Inside is a {name}" (.Name (Utilities|Struct|BreakS_Item (Utilities|Array|Get(acopy) (Variables|/Game/CodingII_Blueprints/BPC_Inventory.BPC_Inventory_C|GetInventory (Variables|Default|GetBPC_Inventory)))))) true true "(R=0.000000,G=0.660000,B=1.000000,A=1.000000)" 9999999.0)
    (CallFunction|OpenChest false)))

(event OnComponentEndOverlap(Sphere)
  (params (OverlappedComponent :type Primitive%20Component%20Object%20Reference) (OtherActor :type Actor%20Object%20Reference) (OtherComp :type Primitive%20Component%20Object%20Reference) (OtherBodyIndex :type Integer))
  (if (Actor|ActorHasTag OtherActor "Player")
    (CallFunction|OpenChest true)))

(event Custom|OpenChest
  (params (Open :type Boolean))
  (if Open
    (bind _open (Timeline|Timeline ReverseFromEnd)
      (:Update
        (Transformation|SetRelativeRotation (Variables|Default|GetHinge) (Math|Rotator|MakeRotator (Math|Float|Lerp 0.0 -7e+01 _open) 0.0 0.0) false false))
      (:Finished
        (if (not Open)
          (Development|PrintText "Show UI")
          (UserInterface|Viewport|AddtoViewport (Variables|Default|GetChestMenu) 0)
          (Default|ShowInventory (stale OnComponentBeginOverlap(Sphere) _asbp_first_person_swap))
          (bind _asgm_save_load (Utilities|Casting|CastToGM_SaveLoad (Game|GetGameMode)))
          (Default|AddInventory (Variables|/Game/CodingII_Blueprints/SaveLoad/GM_SaveLoad.GM_SaveLoad_C|GetLevelState _asgm_save_load) (Variables|Default|GetBPC_Inventory)))))
    (else
      (Timeline|Timeline PlayFromStart))))

(event Custom|Load%20Inventory
  (params (EnumInventory :type Array%20of%20E_Item%20Enums :default "NewEnumerator5"))
  (Variables|/Game/CodingII_Blueprints/BPC_Inventory.BPC_Inventory_C|SetEnumInventory (Variables|Default|GetBPC_Inventory) EnumInventory))

(event Collision|EventActorBeginOverlap
  (params (OtherActor :type Actor%20Object%20Reference)))

(event EventTick
  (params (DeltaSeconds :type Float%20%28single-precision%29)))

(event EventBeginPlay
  (bind _returnvalue (UserInterface|CreateWidget "/Game/Widgets/W_ChestMenu.W_ChestMenu_C" 0 (Variables|Default|GetBPC_Inventory)))
  (Variables|Default|SetChestMenu _returnvalue))

(fn ConstructionScript)