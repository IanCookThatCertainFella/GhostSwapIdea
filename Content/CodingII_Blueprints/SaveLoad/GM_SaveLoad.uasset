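; Game mode that saves and restores player and level state across two save slots.
; BeginPlay loads existing saves or creates new SG_Player and SG_LevelState objects.
; Player slot holds inventories and forward vector; the level-named slot restores actors and player transform, though Save never writes its PlayerTransform input.
; DeleteLevelSave reloads the level but deletes a SlotName_Level slot, unlike the plain level name used for saving.
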(event EventBeginPlay
  (Utilities|FlowControl|Sequence
    (:then_0
      (Development|PrintString "Start!")
      (bind _returnvalue (SaveGame|DoesSaveGameExist (Variables|Default|GetSlotName)))
      (if _returnvalue
        (Utilities|FlowControl|Delay 0.2)
        (CallFunction|Load)
        (else
          (bind _returnvalue_2 (SaveGame|CreateSaveGameObject "/Game/CodingII_Blueprints/SaveLoad/SG_Player.SG_Player_C"))
          (Variables|Default|SetPlayerSave _returnvalue_2)
          (Development|PrintString "Make Save!"))))
    (:then_1
      (bind _returnvalue_3 (Game|GetCurrentLevelName true))
      (bind _returnvalue_4 (SaveGame|DoesSaveGameExist _returnvalue_3))
      (if _returnvalue_4
        (CallFunction|Load)
        (else
          (bind _returnvalue_5 (SaveGame|CreateSaveGameObject "/Game/CodingII_Blueprints/SaveLoad/SG_LevelState.SG_LevelState_C"))
          (Variables|Default|SetLevelState _returnvalue_5))))))

(event EventTick
  (params (DeltaSeconds :type Float%20%28single-precision%29)))

(fn ConstructionScript)

(fn Save
  (params (Belt :type Array%20of%20E_Item%20Enums :default "NewEnumerator5") (Player%20Inv :type Array%20of%20E_Item%20Enums :default "NewEnumerator5") (Player%20Transform :type Transform) (Forward%20Vector :type Vector))
  (bind _playersave (Variables|Default|GetPlayerSave))
  (Utilities|FlowControl|Sequence
    (:then_0
      ;[0.15 0.15 0.15 0.5] Saving Player Stuff
      (Variables|/Game/CodingII_Blueprints/SaveLoad/SG_Player.SG_Player_C|SetBelt _playersave Belt)
      (Variables|/Game/CodingII_Blueprints/SaveLoad/SG_Player.SG_Player_C|SetBackpack _playersave Player%20Inv)
      (Variables|/Game/CodingII_Blueprints/SaveLoad/SG_Player.SG_Player_C|SetForward _playersave Forward%20Vector)
      (SaveGame|SaveGametoSlot (Variables|Default|GetPlayerSave) (Variables|Default|GetSlotName)))
    (:then_1
      ;[0.15 0.15 0.15 0.5] Saving Level Stuff
      (Variables|/Game/CodingII_Blueprints/SaveLoad/SG_LevelState.SG_LevelState_C|SetPlayerTransform (Variables|Default|GetLevelState) "")
      (bind _returnvalue (Game|GetCurrentLevelName true))
      (bind _returnvalue_2 (SaveGame|SaveGametoSlot (Variables|Default|GetLevelState) _returnvalue))
      (if _returnvalue_2
        (Development|PrintString "Save the Game!")
        (else
          (Development|PrintString "Did not a save!"))))))

(fn Load
  (Utilities|FlowControl|Sequence
    (:then_0
      (bind _returnvalue (SaveGame|LoadGamefromSlot (Variables|Default|GetSlotName)))
      (bind _assg_player (Utilities|Casting|CastToSG_Player _returnvalue))
      (Variables|Default|SetPlayerSave _assg_player)
      (bind _asbp_first_person_swap (Utilities|Casting|CastToBP_FirstPersonSwap (Game|GetPlayerCharacter 0)))
      (Default|SetInventory (Variables|/Game/CodingII_Blueprints/BP_FirstPersonSwap.BP_FirstPersonSwap_C|GetBPC_BackPack _asbp_first_person_swap) (Variables|/Game/CodingII_Blueprints/SaveLoad/SG_Player.SG_Player_C|GetBackpack (Variables|Default|GetPlayerSave)))
      (Default|SetInventory (Variables|/Game/CodingII_Blueprints/BP_FirstPersonSwap.BP_FirstPersonSwap_C|GetBPC_BeltInv _asbp_first_person_swap) (Variables|/Game/CodingII_Blueprints/SaveLoad/SG_Player.SG_Player_C|GetBelt (Variables|Default|GetPlayerSave)))
      (Development|PrintText "Load!"))
    (:then_1
      (bind _returnvalue_2 (Game|GetCurrentLevelName true))
      (bind _returnvalue_3 (SaveGame|LoadGamefromSlot _returnvalue_2))
      (bind _assg_level_state (Utilities|Casting|CastToSG_LevelState _returnvalue_3))
      (bind _output_get (Variables|Default|SetLevelState _assg_level_state))
      (Default|ActivateActors _output_get)
      (bind _asbp_first_person_swap_2 (Utilities|Casting|CastToBP_FirstPersonSwap (Game|GetPlayerCharacter 0)))
      (Default|LoadTransform _asbp_first_person_swap_2 (Variables|/Game/CodingII_Blueprints/SaveLoad/SG_LevelState.SG_LevelState_C|GetPlayerTransform (Variables|Default|GetLevelState)) "0, 0, 0")
      (Pawn|SetControlRotation (Game|GetPlayerController 0) (.Rotation (Math|Transform|BreakTransform (Variables|/Game/CodingII_Blueprints/SaveLoad/SG_LevelState.SG_LevelState_C|GetPlayerTransform (Variables|Default|GetLevelState))))))))

(fn DeleteSave
  (SaveGame|DeleteGameinSlot (Variables|Default|GetSlotName))
  (CallFunction|DeleteLevelSave))

(fn DeleteLevelSave
  (bind _returnvalue (Game|GetCurrentLevelName true))
  (SaveGame|DeleteGameinSlot (Utilities|String|Append (Variables|Default|GetSlotName) "_" _returnvalue))
  (Game|OpenLevel(byName) (Utilities|String|StringToName _returnvalue)))