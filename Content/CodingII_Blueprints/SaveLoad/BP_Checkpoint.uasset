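; BP_Checkpoint is a checkpoint actor that saves the player's progress when the first-person character overlaps it.
; On BeginPlay it casts and caches the GM_SaveLoad game mode.
; On overlap with a BP_FirstPersonSwap, it passes the belt and backpack inventories, player transform and forward vector to the game mode's Save function, then prints a confirmation message.
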(event EventBeginPlay
  (bind _asgm_save_load (Utilities|Casting|CastToGM_SaveLoad (Game|GetGameMode)))
  (Variables|Default|SetGame%20Mode _asgm_save_load))

(event Collision|EventActorBeginOverlap
  (params (OtherActor :type Actor%20Object%20Reference))
  (bind _asbp_first_person_swap (Utilities|Casting|CastToBP_FirstPersonSwap OtherActor))
  (Default|Save (Variables|Default|GetGame%20Mode) (Variables|/Game/CodingII_Blueprints/BPC_Inventory.BPC_Inventory_C|GetEnumInventory (Variables|/Game/CodingII_Blueprints/BP_FirstPersonSwap.BP_FirstPersonSwap_C|GetBPC_BeltInv _asbp_first_person_swap)) (Variables|/Game/CodingII_Blueprints/BPC_Inventory.BPC_Inventory_C|GetEnumInventory (Variables|/Game/CodingII_Blueprints/BP_FirstPersonSwap.BP_FirstPersonSwap_C|GetBPC_BackPack _asbp_first_person_swap)) (Transformation|GetActorTransform _asbp_first_person_swap) (Transformation|GetActorForwardVector _asbp_first_person_swap))
  (Development|PrintText "Checkpoint, yeah!"))

(event EventTick
  (params (DeltaSeconds :type Float%20%28single-precision%29)))

(fn ConstructionScript)