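; BP_Key is a pickup key item that removes a BP_Door when used on it.
; Pickup stores the owner, disables box collision and returns the item type, while Drop clears the owner's held item and restores collision and physics with a zero-valued impulse.
; Use runs a short, debug-drawn visibility trace along the box's forward vector, destroying both door and key on a hit, otherwise printing the hit actor's name.
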(event EventBeginPlay)

(event Collision|EventActorBeginOverlap
  (params (OtherActor :type Actor%20Object%20Reference)))

(event EventTick
  (params (DeltaSeconds :type Float%20%28single-precision%29)))

(event EventAlternateUse)

(event EventUse
  (bind _box (Variables|Default|GetBox))
  (bind _returnvalue (Transformation|GetWorldLocation _box))
  (bind _outhit (Collision|LineTraceByChannel _returnvalue (+ _returnvalue (* (Math|Vector|GetForwardVector _box) 3e+02)) "TraceTypeQuery1" false 0 "Persistent"))
  (bind _asbp_door (Utilities|Casting|CastToBP_Door (.HitActor (Collision|BreakHitResult _outhit)))
    (:then
      (Variables|/Game/CodingII_Blueprints/BPC_Interact.BPC_Interact_C|SetCurrently%20Held%20Item (Variables|Default|GetOwner1) 0) ; Set "Currently Held Item" to nothing
      (Actor|DestroyActor _asbp_door))
    (:CastFailed
      (Development|PrintString (Utilities|GetDisplayName (.HitActor (Collision|BreakHitResult _outhit)))))))

(event EventDrop
  (bind _box (Variables|Default|GetBox))
  (Variables|/Game/CodingII_Blueprints/BPC_Interact.BPC_Interact_C|SetCurrently%20Held%20Item (Variables|Default|GetOwner1) 0) ; Set "Currently Held Item" to nothing
  (Collision|SetCollisionEnabled _box "QueryAndPhysics")
  (Physics|SetSimulatePhysics _box true)
  (Physics|AddImpulse _box (* "" "") "None" true))

(fn ConstructionScript)

(fn Pickup
  (params (Owner :type BPC%20Interact%20Object%20Reference))
  (Variables|Default|SetOwner1 Owner)
  (Collision|SetCollisionEnabled (Variables|Default|GetBox) "NoCollision")
  (return (Variables|Default|GetItem%20Type)))