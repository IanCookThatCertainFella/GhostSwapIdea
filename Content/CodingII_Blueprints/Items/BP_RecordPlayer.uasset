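; BP_RecordPlayer is a pickup item that plays audio on Use and stops it on AlternateUse.
; Pickup stores the owner, disables box collision, registers the actor in the GM_SaveLoad level state and returns its item type.
; Drop clears the owner's held item and restores collision and physics, though its impulse evaluates to zero.
; Activate destroys the actor.
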(event EventBeginPlay)

(event Collision|EventActorBeginOverlap
  (params (OtherActor :type Actor%20Object%20Reference)))

(event EventTick
  (params (DeltaSeconds :type Float%20%28single-precision%29)))

(event EventAlternateUse
  (Audio|Components|Audio|Stop (Variables|Default|GetAudio)))

(event EventUse
  (Audio|Components|Audio|Play (Variables|Default|GetAudio) 0.0))

(event EventActivate
  (Actor|DestroyActor))

(event EventDrop
  (bind _box (Variables|Default|GetBox))
  (Variables|/Game/CodingII_Blueprints/BPC_Interact.BPC_Interact_C|SetCurrently%20Held%20Item (Variables|Default|GetOwner_0) 0) ; Set "Currently Held Item" to nothing
  (Collision|SetCollisionEnabled _box "QueryAndPhysics")
  (Physics|SetSimulatePhysics _box true)
  (Physics|AddImpulse _box (* "" "") "None" true))

(fn ConstructionScript)

(fn Pickup
  (params (Owner :type BPC%20Interact%20Object%20Reference))
  (Variables|Default|SetOwner_0 Owner)
  (Collision|SetCollisionEnabled (Variables|Default|GetBox) "NoCollision")
  (bind _asgm_save_load (Utilities|Casting|CastToGM_SaveLoad (Game|GetGameMode)))
  (Default|AddActor (Variables|/Game/CodingII_Blueprints/SaveLoad/GM_SaveLoad.GM_SaveLoad_C|GetLevelState _asgm_save_load) self)
  (return (Variables|Default|GetItemType)))