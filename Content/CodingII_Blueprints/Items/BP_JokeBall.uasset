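; BP_JokeBall is a holdable item that shows a Joke widget on screen when used.
; Pickup stores the owner, disables the sphere's collision and returns the item type.
; Drop clears the owner's held item and restores collision and physics, though its impulse evaluates to zero.
; Alternate use only prints a debug string.
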(event Custom|Pickup_1_1
  (params (Owner :type BPC%20Interact%20Object%20Reference))
  (Collision|SetCollisionEnabled (Variables|Default|GetSphere1) "NoCollision"))

(event EventBeginPlay)

(event Collision|EventActorBeginOverlap
  (params (OtherActor :type Actor%20Object%20Reference)))

(event EventTick
  (params (DeltaSeconds :type Float%20%28single-precision%29)))

(event EventAlternateUse
  (Development|PrintString "Da Funny"))

(event EventUse
  (bind _returnvalue (UserInterface|CreateWidget (Variables|Default|GetJoke) (Game|GetPlayerController 0)))
  (UserInterface|Viewport|AddtoViewport _returnvalue 0))

(event EventDrop
  (bind _sphere1 (Variables|Default|GetSphere1))
  (Variables|/Game/CodingII_Blueprints/BPC_Interact.BPC_Interact_C|SetCurrently%20Held%20Item (stale Custom|Pickup_1_1 Owner) 0) ; Set "Currently Held Item" to nothing
  (Collision|SetCollisionEnabled _sphere1 "QueryAndPhysics")
  (Physics|SetSimulatePhysics _sphere1 true)
  (Physics|AddImpulse _sphere1 (* "" "") "None" true))

(fn ConstructionScript)

(fn Pickup
  (params (Owner :type BPC%20Interact%20Object%20Reference))
  (Variables|Default|SetOwner_0 Owner)
  (Collision|SetCollisionEnabled (Variables|Default|GetSphere1) "NoCollision")
  (return (Variables|Default|GetItem%20Type)))