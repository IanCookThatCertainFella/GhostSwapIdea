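; BP_ThrownBoomerang is a flying, AI-moved character acting as Link's thrown boomerang, looping a timeline to spin its mesh.
; Fly sets speed and acceleration, then chains AIMoveTo without pathfinding through Link's targets before returning to Link.
; Capsule overlaps count "Target" hits with indexed sounds, or despawn it on "Block" actors.
; Despawn destroys it, clears Link's throw state and "Marked" tags, and calls Catch.
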(event OnComponentBeginOverlap(CapsuleComponent)
  (params (OverlappedComponent :type Primitive%20Component%20Object%20Reference) (OtherActor :type Actor%20Object%20Reference) (OtherComp :type Primitive%20Component%20Object%20Reference) (OtherBodyIndex :type Integer) (bFromSweep :type Boolean) (SweepResult :type Hit%20Result%20Structure%20%28by%20ref%29))
  (bind _link (Variables|Default|GetLink))
  (if (Actor|ActorHasTag OtherActor "Block")
    (CallFunction|Despawn)
    (elif (Actor|ActorHasTag OtherActor "Target")
      (Variables|/Game/CodingII_Blueprints/Items/BP_Boomerang_Interactible.BP_Boomerang_Interactible_C|SetHitTargets _link (+ (Variables|/Game/CodingII_Blueprints/Items/BP_Boomerang_Interactible.BP_Boomerang_Interactible_C|GetHitTargets _link) 1))
      (Audio|PlaySound2D (Utilities|Array|Get(acopy) (Variables|Default|GetHitSounds) (Variables|Default|GetCurrentTarget)) 1.0 1.0 0.0 0 0))))

(event Custom|Fly
  (params (TargetNumber :type Integer) (Speed :type Float%20%28double-precision%29) (Acceleration :type Float%20%28double-precision%29))
  (bind _charactermovement (Variables|Character|GetCharacterMovement))
  (Variables|/Script/Engine.CharacterMovementComponent|SetMaxFlySpeed _charactermovement Speed)
  (Variables|/Script/Engine.CharacterMovementComponent|SetMaxAcceleration _charactermovement Acceleration)
  (Development|PrintString (Utilities|GetDisplayName (Utilities|Array|Get(acopy) (Variables|/Game/CodingII_Blueprints/Items/BP_Boomerang_Interactible.BP_Boomerang_Interactible_C|GetTargets (Variables|Default|GetLink)) (Variables|Default|GetCurrentTarget))))
  (Variables|Default|SetTargetAmounts TargetNumber)
  (AI|AIMoveTo (AI|GetAIController self) "0, 0, 0" (Utilities|Array|Get(acopy) (Variables|/Game/CodingII_Blueprints/Items/BP_Boomerang_Interactible.BP_Boomerang_Interactible_C|GetTargets (Variables|Default|GetLink)) (Variables|Default|GetCurrentTarget)) 1.0 "Default" "Default" false true :!label _label
    (:then
      (Development|PrintString "I'm going!"))
    (:OnRequestFailed
      (Development|PrintString "Can't Make it!"))
    (:OnMoveFinished
      (Variables|Default|SetCurrentTarget (+ (Variables|Default|GetCurrentTarget) 1))
      (if (> (+ (Variables|Default|GetCurrentTarget) 1) (Variables|Default|GetTargetAmounts))
        (CallFunction|Return)
        (else
          (goto _label))))))

(event Custom|Despawn
  (bind _link (Variables|Default|GetLink))
  (bind _link_2 (Variables|Default|GetLink))
  (Actor|DestroyActor)
  (Variables|/Game/CodingII_Blueprints/Items/BP_Boomerang_Interactible.BP_Boomerang_Interactible_C|SetHitTargets _link 0)
  (Variables|/Game/CodingII_Blueprints/Items/BP_Boomerang_Interactible.BP_Boomerang_Interactible_C|SetThrown _link false)
  (Variables|/Game/CodingII_Blueprints/Items/BP_Boomerang_Interactible.BP_Boomerang_Interactible_C|SetTargetNumber _link 0)
  (for _array_element (Variables|/Game/CodingII_Blueprints/Items/BP_Boomerang_Interactible.BP_Boomerang_Interactible_C|GetTargets _link)
    (bind _returnvalue (Utilities|Array|RemoveItem (Variables|/Script/Engine.Actor|GetTags _array_element) "Marked"))
    (if _returnvalue
      (Development|PrintString "Yahoo!")
      (else
        (Development|PrintString "No!"))))
  (Utilities|Array|Clear (Variables|/Game/CodingII_Blueprints/Items/BP_Boomerang_Interactible.BP_Boomerang_Interactible_C|GetTargets _link_2))
  (Development|PrintString "Done!")
  (Default|Catch _link_2))

(event Custom|Return
  (AI|AIMoveTo (AI|GetAIController self) "0, 0, 0" (Variables|Default|GetLink) 1.0 "Default" "Default" false true
    (:OnRequestFailed
      (CallFunction|Despawn)
      (Development|PrintString "Can't Make it!"))
    (:OnMoveFinished
      (if (== (Variables|/Game/CodingII_Blueprints/Items/BP_Boomerang_Interactible.BP_Boomerang_Interactible_C|GetHitTargets (Variables|Default|GetLink)) 5)
        _
        (elif (> 0 5)
          _
          (else
            _)))
      (CallFunction|Despawn))))

(event EventBeginPlay
  (bind _rotate (Timeline|Spinning PlayFromStart)
    (:Update
      (Transformation|SetRelativeRotation (Variables|Default|GetSphere) (Math|Rotator|MakeRotator 0.0 0.0 (Math|Float|Lerp 0.0 3.6e+02 _rotate)) false false))
    (:Finished
      (Timeline|Spinning PlayFromStart))))

(event Collision|EventActorBeginOverlap
  (params (OtherActor :type Actor%20Object%20Reference)))

(event EventTick
  (params (DeltaSeconds :type Float%20%28single-precision%29)))

(fn ConstructionScript)