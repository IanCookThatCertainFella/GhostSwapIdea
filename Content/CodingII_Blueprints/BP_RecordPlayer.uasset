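; BP_RecordPlayer is a record player item that can be picked up, dropped and used to play audio.
; Use starts the Audio component from the beginning, and AlternateUse stops it.
; Pickup disables Box collision, while Drop clears the owner's held item, restores collision and enables physics.
; The impulse applied on drop evaluates to zero as written.
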(event EventBeginPlay)

(event Collision|EventActorBeginOverlap
  (params (OtherActor :type Actor%20Object%20Reference)))

(event EventTick
  (params (DeltaSeconds :type Float%20%28single-precision%29)))

(event EventAlternateUse
  (Audio|Components|Audio|Stop (Variables|Default|GetAudio)))

(event EventUse
  (Audio|Components|Audio|Play (Variables|Default|GetAudio) 0.0))

(event EventPickup
  (params (Owner :type BPC%20Interact%20Object%20Reference))
  (Collision|SetCollisionEnabled (Variables|Default|GetBox) "NoCollision"))

(event EventDrop
  (bind _box (Variables|Default|GetBox))
  (Variables|/Game/CodingII_Blueprints/BPC_Interact.BPC_Interact_C|SetCurrently%20Held%20Item (stale EventPickup Owner) 0) ; Set "Currently Held Item" to nothing
  (Collision|SetCollisionEnabled _box "QueryAndPhysics")
  (Physics|SetSimulatePhysics _box true)
  (Physics|AddImpulse _box (* "" "") "None" true))

(fn ConstructionScript)