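; BP_Ranged is an AI pawn, ranged by its name, that takes damage, can be healed and destroys itself when health runs out.
; It caches its AIC_Base controller on BeginPlay.
; AnyDamage reports a damage event at the instigator pawn's location for AI perception, sends a TookDamage event to the controller's StateTree, then subtracts Health.
; GetHealthKit adds health, clamped between zero and one.
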(event Custom|Get%20HealthKit
  (params (Health :type Float%20%28double-precision%29))
  (Variables|Default|SetHealth (Math|Float|Clamp(Float) (+ (Variables|Default|GetHealth) Health))))

(event Collision|EventActorBeginOverlap
  (params (OtherActor :type Actor%20Object%20Reference)))

(event EventTick
  (params (DeltaSeconds :type Float%20%28single-precision%29)))

(event Game|Damage|EventAnyDamage
  (params (Damage :type Float%20%28single-precision%29) (DamageType :type Damage%20Type%20Object%20Reference) (InstigatedBy :type Controller%20Object%20Reference) (DamageCauser :type Actor%20Object%20Reference))
  (Class|AISenseDamage|ReportDamageEvent self InstigatedBy Damage (Transformation|GetActorLocation (Pawn|GetControlledPawn InstigatedBy)) "0, 0, 0" "None")
  (Gameplay|StateTree|SendStateTreeEvent (Variables|/Game/CodingII_Blueprints/AI/AIC_Base.AIC_Base_C|GetStateTreeAI (Variables|Default|GetAs%20AIC%20Base)) (Utilities|Struct|MakeStateTreeEvent "(TagName=\"AI.Event.TookDamage\")") :!class /Script/GameplayStateTreeModule.StateTreeComponent)
  (bind _output_get (Variables|Default|SetHealth (- (Variables|Default|GetHealth) Damage)))
  (if (not (> _output_get 0.0))
    (Development|PrintString "I'm Dead, AHH")
    (Actor|DestroyActor)))

(event EventBeginPlay
  (bind _asaic_base (Utilities|Casting|CastToAIC_Base (Pawn|GetController)))
  (Variables|Default|SetAs%20AIC%20Base _asaic_base))

(fn ConstructionScript)