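; AI turret that turns to face a sensed target and fires BP_Bullet projectiles at it.
; HandleSight stores the target and starts Tracking, or calls Looking when sight fails, which only stops the per-tick look-at rotation.
; Tracking and Attacking call each other through a one-second Delay, so firing repeats even after sight is lost.
; Each shot spawns at BulletSpawn and gets a forward velocity impulse.
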(event Custom|Fire%20Projectile
  (bind _bulletspawn (Variables|Default|GetBulletSpawn))
  (bind _returnvalue (Game|SpawnActorfromClass "/Game/CodingII_Blueprints/BP_Bullet.BP_Bullet_C" (Transformation|GetWorldTransform _bulletspawn) "Undefined" "MultiplyWithRoot" 0 0))
  (Physics|AddImpulse (Variables|/Game/CodingII_Blueprints/BP_Bullet.BP_Bullet_C|GetSphere _returnvalue) (* (Math|Vector|GetForwardVector _bulletspawn) 3e+03) "None" true))

(event Custom|Looking
  (Variables|Default|SetTrackingTarget false))

(event Custom|Tracking
  (Variables|Default|SetTrackingTarget true)
  (Utilities|FlowControl|Delay 1.0)
  (CallFunction|Attacking))

(event Custom|Attacking
  (CallFunction|FireProjectile)
  (CallFunction|Tracking))

(event Custom|Handle%20Sight
  (params (Target :type Actor%20Object%20Reference) (Successfully%20Sensed :type Boolean))
  (if Successfully%20Sensed
    (Variables|Default|SetTarget Target)
    (CallFunction|Tracking)
    (else
      (CallFunction|Looking))))

(event EventBeginPlay)

(event Collision|EventActorBeginOverlap
  (params (OtherActor :type Actor%20Object%20Reference)))

(event EventTick
  (params (DeltaSeconds :type Float%20%28single-precision%29))
  (if (Variables|Default|GetTrackingTarget)
    (Transformation|SetActorRotation (Math|Rotator|FindLookatRotation (Transformation|GetActorLocation) (Transformation|GetActorLocation (Variables|Default|GetTarget))))))

(fn ConstructionScript)