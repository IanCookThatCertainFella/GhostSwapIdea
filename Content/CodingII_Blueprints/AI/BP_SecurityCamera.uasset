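; BP_SecurityCamera is an AI security camera that raises an alarm when it sees a target.
; HandleSight swaps the mesh material and prints a message for both sighted and lost states.
; On a sighting it plays a jazz sound and sends the location to every BP_ReallyDumbAI through CheckOutAlarm.
; Nothing in the event graph calls HandleSight; its forget-target and stimulus-class fragments never run.
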(event EventBeginPlay)

(event Collision|EventActorBeginOverlap
  (params (OtherActor :type Actor%20Object%20Reference)))

(event EventTick
  (params (DeltaSeconds :type Float%20%28single-precision%29)))

(fn ConstructionScript)

(fn HandleSight
  (params (DaTarget :type Actor%20Object%20Reference) (SuccessfullySensed :type Boolean) (Location :type Vector))
  (bind _staticmesh (Variables|Default|GetStaticMesh))
  (if SuccessfullySensed
    (Development|PrintString "I saw him! I saw him!")
    (Rendering|Material|SetMaterial _staticmesh 0 "/Engine/Engine_MI_Shaders/Instances/M_Shader_SimpleTranslucent_Invis.M_Shader_SimpleTranslucent_Invis")
    (Audio|PlaySoundatLocation "/Game/Audio/RecordMusicCues/20s_Jazz.20s_Jazz" (Transformation|GetActorLocation) "0, 0, 0" 1.0 1.0 0.0 "/Game/Audio/DefaultAttenuation.DefaultAttenuation" 0 0 0)
    (bind _outactors (Actor|GetAllActorsOfClass "/Game/CodingII_Blueprints/AI/BP_ReallyDumbAI.BP_ReallyDumbAI_C"))
    (for _array_element _outactors
      (Default|CheckOutAlarm _array_element Location))
    (else
      (Development|PrintString "Where'd he go?")
      (Rendering|Material|SetMaterial _staticmesh 0 "/Engine/EditorMaterials/Cross_Mat.Cross_Mat"))))