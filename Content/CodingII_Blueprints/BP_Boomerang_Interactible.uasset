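; Holdable boomerang pickup that marks multiple targets while aiming, then throws at them.
; Use starts a repeating camera line trace that tags hit "Target" actors as "Marked" and adds them to a list.
; AlternateUse stops aiming and, given targets and no earlier throw, hides the item and spawns a linked BP_ItemBoomerang to fly.
; Catch unhides the item but leaves Thrown set; Drop, blocked while aiming, restores collision and physics.
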(event Custom|Catch
  (Rendering|SetActorHiddenInGame false))

(event Custom|Loop
  (bind _thrower (Variables|Default|GetThrower))
  (bind _firstpersoncamera (Variables|/Game/CodingII_Blueprints/BP_FirstPersonSwap.BP_FirstPersonSwap_C|GetFirstPersonCamera _thrower))
  (bind _returnvalue (Transformation|GetWorldLocation _firstpersoncamera))
  (Utilities|FlowControl|Delay (Variables|Default|GetDuration))
  (bind _outhit (Collision|LineTraceForObjects _returnvalue (+ _returnvalue (* (Math|Vector|GetForwardVector _firstpersoncamera) 2e+03)) (Utilities|Array|MakeArray "ObjectTypeQuery2" "ObjectTypeQuery1" "ObjectTypeQuery3") false (Utilities|Array|MakeArray (Variables|Default|GetThrower)) "ForDuration"))
  (Utilities|IsValid (.HitActor (Collision|BreakHitResult _outhit))
    (:Is%20Valid
      (if (Actor|ActorHasTag (.HitActor (Collision|BreakHitResult _outhit)) "Target")
        (if (Actor|ActorHasTag (.HitActor (Collision|BreakHitResult _outhit)) "Marked")
          (Development|PrintString "You're marked!")
          (else
            (Utilities|Array|Add (Variables|Default|GetTargets) (.HitActor (Collision|BreakHitResult _outhit)))
            (Utilities|Array|Add (Variables|/Script/Engine.Actor|GetTags (.HitActor (Collision|BreakHitResult _outhit))) "Marked")
            (Variables|Default|SetTargetNumber (+ (Variables|Default|GetTargetNumber) 1))))))
    (:Is%20Not%20Valid
      _))
  (if (Variables|Default|GetbAiming)
    (CallFunction|Loop)))

(event EventBeginPlay)

(event Collision|EventActorBeginOverlap
  (params (OtherActor :type Actor%20Object%20Reference)))

(event EventTick
  (params (DeltaSeconds :type Float%20%28single-precision%29)))

(event EventUse
  (bind _thrower (Variables|Default|GetThrower))
  (bind _firstpersoncamera (Variables|/Game/CodingII_Blueprints/BP_FirstPersonSwap.BP_FirstPersonSwap_C|GetFirstPersonCamera _thrower))
  (bind _returnvalue (Transformation|GetWorldLocation _firstpersoncamera))
  (Variables|Default|SetbAiming true)
  (bind _outhit (Collision|LineTraceForObjects _returnvalue (+ _returnvalue (* (Math|Vector|GetForwardVector _firstpersoncamera) 2e+03)) (Utilities|Array|MakeArray "ObjectTypeQuery2" "ObjectTypeQuery1" "ObjectTypeQuery3") false (Utilities|Array|MakeArray (Variables|Default|GetThrower)) "ForDuration"))
  (Utilities|IsValid (.HitActor (Collision|BreakHitResult _outhit))
    (:Is%20Valid
      (if (Actor|ActorHasTag (.HitActor (Collision|BreakHitResult _outhit)) "Target")
        (if (Actor|ActorHasTag (.HitActor (Collision|BreakHitResult _outhit)) "Marked")
          (Development|PrintString "You're marked!")
          (else
            (Utilities|Array|Add (Variables|Default|GetTargets) (.HitActor (Collision|BreakHitResult _outhit)))
            (Utilities|Array|Add (Variables|/Script/Engine.Actor|GetTags (.HitActor (Collision|BreakHitResult _outhit))) "Marked")
            (Variables|Default|SetTargetNumber (+ (Variables|Default|GetTargetNumber) 1))))))
    (:Is%20Not%20Valid
      _))
  (if (Variables|Default|GetbAiming)
    (CallFunction|Loop)))

(event EventPickup
  (params (Owner :type BPC%20Interact%20Object%20Reference))
  (Variables|Default|SetThrower (Variables|/Game/CodingII_Blueprints/BPC_Interact.BPC_Interact_C|GetPlayer Owner))
  (Collision|SetCollisionEnabled (Variables|Default|GetBox) "NoCollision"))

(event EventDrop
  (bind _box (Variables|Default|GetBox))
  (if (not (Variables|Default|GetbAiming))
    (Variables|Default|SetThrower 0)
    (Variables|/Game/CodingII_Blueprints/BPC_Interact.BPC_Interact_C|SetCurrently%20Held%20Item (stale EventPickup Owner) 0) ; Set "Currently Held Item" to nothing
    (Collision|SetCollisionEnabled _box "QueryAndPhysics")
    (Physics|SetSimulatePhysics _box true)
    (Physics|AddImpulse _box (* "" "") "None" true)))

(event EventAlternateUse
  (bind _thrower (Variables|Default|GetThrower))
  (bind _firstpersoncamera (Variables|/Game/CodingII_Blueprints/BP_FirstPersonSwap.BP_FirstPersonSwap_C|GetFirstPersonCamera _thrower))
  (Variables|Default|SetbAiming false)
  (if (and (> (Variables|Default|GetTargetNumber) 0) (!= (Variables|Default|GetThrown) true))
    (Rendering|SetActorHiddenInGame true)
    (Variables|Default|SetThrown true)
    (bind _returnvalue (Game|SpawnActorfromClass "/Game/CodingII_Blueprints/BP_ItemBoomerang.BP_ItemBoomerang_C" (Math|Transform|MakeTransform (+ (Transformation|GetWorldLocation _firstpersoncamera) (* (Math|Vector|GetForwardVector _firstpersoncamera) 2e+01)) "0, 0, 0" "1.000000,1.000000,1.000000") "Undefined" "MultiplyWithRoot" 0 0))
    (Variables|/Game/CodingII_Blueprints/BP_ItemBoomerang.BP_ItemBoomerang_C|SetLink _returnvalue self)
    (Default|Fly _returnvalue (Variables|Default|GetTargetNumber))
    (Development|PrintString (Utilities|GetDisplayName (Utilities|Array|Get(acopy) (Variables|Default|GetTargets))))
    (else
      (Development|PrintString "Get somebody!"))))

(fn ConstructionScript)