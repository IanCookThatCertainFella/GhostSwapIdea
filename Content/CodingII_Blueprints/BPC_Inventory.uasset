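; Inventory component that stores items as an array of item enums and looks up their data in the DT_Items data table.
; GetSlot resolves a slot's enum through GetItemDetails, which scans every table row for a matching enum.
; SetSlot writes one entry and fires OnSlotUpdated, while SetInventory replaces the whole array and fires RefreshGrid for listeners.
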(event EventBeginPlay)

(event EventTick
  (params (DeltaSeconds :type Float%20%28single-precision%29)))

(fn GetItemDetails
  (params (Requested%20Item :type E_Item%20Enum :default "NewEnumerator0"))
  (bind _outrownames (DataTable|GetDataTableRowNames "/Game/CodingII_Blueprints/DataTables/DT_Items.DT_Items"))
  (for _array_element _outrownames
    (bind _returnvalue (Utilities|GetDataTableRow "/Game/CodingII_Blueprints/DataTables/DT_Items.DT_Items" _array_element)
      (:then
        (if (Utilities|Enum|Equal(Enum) (.Enum (Utilities|Struct|BreakS_Item _returnvalue)) Requested%20Item)
          (return _returnvalue))))))

(fn GetSlot
  (params (Requested%20Slot :type Integer))
  (bind _item_details (CallFunction|GetItemDetails (Utilities|Array|Get(acopy) (Variables|Default|GetEnumInventory) Requested%20Slot)))
  (return _item_details))

(fn SetSlot
  (params (Item :type E_Item%20Enum :default "NewEnumerator5") (Slot%20Index :type Integer))
  (Utilities|Array|SetArrayElem (Variables|Default|GetEnumInventory) Slot%20Index Item)
  (Default|CallOnSlotUpdated Slot%20Index))

(fn SetInventory
  (params (Enum%20Inv :type Array%20of%20E_Item%20Enums :default "NewEnumerator5"))
  (Variables|Default|SetEnumInventory Enum%20Inv)
  (Default|CallRefreshGrid))