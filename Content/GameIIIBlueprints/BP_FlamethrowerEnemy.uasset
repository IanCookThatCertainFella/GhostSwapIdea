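; Flamethrower enemy Blueprint that times its shot delay to the music tempo.
; The Construction Script reads BPM from the Metronome and sets ShotDelay to one third of a beat, then runs the parent construction script.
; BeginPlay only calls the parent, and Tick and overlap are disabled stubs, so this Blueprint adds no other behavior of its own.
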(event EventBeginPlay
  (|CallParentFunction))

(event Collision|EventActorBeginOverlap
  (params (OtherActor :type Actor%20Object%20Reference))
  (|CallParentFunction OtherActor) ; This node is disabled and will not be called.\nDrag off pins to build functionality.
)

(event EventTick
  (params (DeltaSeconds :type Float%20%28single-precision%29))
  (|CallParentFunction DeltaSeconds) ; This node is disabled and will not be called.\nDrag off pins to build functionality.
)

(fn ConstructionScript
  (Variables|Default|SetShotDelay (Utilities|Operators|Divide 6e+01 (Variables|/Game/GameIIIBlueprints/BP_Enemy_Metronome.BP_Enemy_Metronome_C|GetBPM (Variables|Default|GetMetronome)) 3.0))
  (|CallParentFunction))