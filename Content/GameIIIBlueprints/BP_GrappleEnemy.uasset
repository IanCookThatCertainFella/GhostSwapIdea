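; Grappling-hook enemy that spots the player, turns to face them, hooks them and pulls itself in to strike.
; Externally triggered Action steps through draw, fire, grapple and reset/stall states.
; Fire line-traces forward and animates the cable by timeline, homing on the player if near the trace point.
; Sphere overlap attaches the hook, a second timeline lerps the enemy to the player, and Swing overlap sends damage and detaches.
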(event OnSeePawn(PawnSensing)
  (params (Pawn :type Pawn%20Object%20Reference))
  (if (Actor|ActorHasTag Pawn "Player")
    (Variables|Default|SetPlayer Pawn)
    (Variables|Default|SetbSeePlayer true)))

(event OnComponentBeginOverlap(Sphere1)
  (params (OverlappedComponent :type Primitive%20Component%20Object%20Reference) (OtherActor :type Actor%20Object%20Reference) (OtherComp :type Primitive%20Component%20Object%20Reference) (OtherBodyIndex :type Integer) (bFromSweep :type Boolean) (SweepResult :type Hit%20Result%20Structure%20%28by%20ref%29))
  (if (Actor|ActorHasTag OtherActor "Player")
    (Variables|Default|SetbPlayerInRange true)
    (Transformation|SetActorRotation (Math|Rotator|FindLookatRotation (Transformation|GetActorLocation) (Transformation|GetActorLocation (Game|Player|GetPlayerPawn 0))) true)))

(event OnComponentEndOverlap(Sphere1)
  (params (OverlappedComponent :type Primitive%20Component%20Object%20Reference) (OtherActor :type Actor%20Object%20Reference) (OtherComp :type Primitive%20Component%20Object%20Reference) (OtherBodyIndex :type Integer))
  (if (Actor|ActorHasTag OtherActor "Player")
    (Variables|Default|SetbPlayerInRange false)))

(event OnComponentBeginOverlap(Sphere)
  (params (OverlappedComponent :type Primitive%20Component%20Object%20Reference) (OtherActor :type Actor%20Object%20Reference) (OtherComp :type Primitive%20Component%20Object%20Reference) (OtherBodyIndex :type Integer) (bFromSweep :type Boolean) (SweepResult :type Hit%20Result%20Structure%20%28by%20ref%29))
  (if (Actor|ActorHasTag OtherActor "Player")
    (Development|PrintString "Got 'Em")
    (Audio|PlaySound2D "/Game/Audio/Boomerang_E.Boomerang_E" 1.0 1.0 0.0 0 0)
    (Variables|Default|SetAttached true)))

(event OnComponentBeginOverlap(Swing)
  (params (OverlappedComponent :type Primitive%20Component%20Object%20Reference) (OtherActor :type Actor%20Object%20Reference) (OtherComp :type Primitive%20Component%20Object%20Reference) (OtherBodyIndex :type Integer) (bFromSweep :type Boolean) (SweepResult :type Hit%20Result%20Structure%20%28by%20ref%29))
  (if (Actor|ActorHasTag OtherActor "Player")
    (Class|BPIDamagible|GetDamaged(Message) OtherActor)
    (Variables|Default|SetAttached false)))

(event Custom|Draw
  (Variables|Default|SetDrawn true))

(event Custom|Fire
  (bind _player (Variables|Default|GetPlayer))
  (bind _returnvalue (Transformation|GetActorLocation _player))
  (if (Math|Boolean|ANDBoolean (Variables|Default|GetbSeePlayer) (Variables|Default|GetbPlayerInRange) (not (Variables|Default|GetbHasFired)))
    (if (Variables|Default|GetbCanShoot)
      (Audio|PlaySound2D "/Game/Audio/Boomerang_D.Boomerang_D" 1.0 1.0 0.0 0 0)
      (Variables|Default|SetbHasFired true)
      (bind _grappletarget (CallFunction|FindTarget))
      (Collision|SetCollisionEnabled (Variables|Default|GetSphere) "QueryOnly")
      (Development|SetHiddeninGame (Variables|Default|GetCable) false false)
      (bind _grappletime (Timeline|Timeline PlayFromStart)
        (:Update
          (if (Math|Boolean|ORBoolean (<= (- (.x _returnvalue) (.x _grappletarget)) -5e+02) (>= (- (.x _returnvalue) (.x _grappletarget)) 5e+02) (<= (- (.y _returnvalue) (.y _grappletarget)) -5e+02) (>= (- (.y _returnvalue) (.y _grappletarget)) 5e+02) (<= (- (.z _returnvalue) (.z _grappletarget)) -3e+02) (>= (- (.z _returnvalue) (.z _grappletarget)) 3e+02))
            (Variables|Default|SetFinalTarget (Variables|Default|GetGrappleTarget))
            (else
              (Variables|Default|SetFinalTarget (Transformation|GetActorLocation (Variables|Default|GetPlayer)))))
          (Transformation|SetWorldLocation (Variables|Default|GetCable) (Math|Vector|Lerp(Vector) (Transformation|GetWorldLocation (Variables|Default|GetCable)) (Variables|Default|GetFinalTarget) _grappletime) true false))
        (:Finished
          (Audio|PlaySound2D "/Game/Audio/Boomerang_C.Boomerang_C" 1.0 1.0 0.0 0 0))))))

(event Custom|GrappleTo
  (bind _grappletime (Timeline|Timeline_0 PlayFromStart)
    (:Update
      (if (Variables|Default|GetAttached)
        (Transformation|SetActorLocation (Math|Vector|Lerp(Vector) (Transformation|GetActorLocation) (Transformation|GetActorLocation (Variables|Default|GetPlayer)) _grappletime) false false)))
    (:Finished
      (CallFunction|ResetGrapple))))

(event Custom|ResetGrapple
  (Variables|Default|SetAttached false)
  (Variables|Default|SetbCanShoot false)
  (Variables|Default|SetDrawn false)
  (Development|SetHiddeninGame (Variables|Default|GetCable) true false)
  (Collision|SetCollisionEnabled (Variables|Default|GetSphere) "NoCollision"))

(event Custom|Stall
  (Variables|Default|SetbCanShoot true)
  (Variables|Default|SetbHasFired false))

(event EventBeginPlay)

(event Collision|EventActorBeginOverlap
  (params (OtherActor :type Actor%20Object%20Reference)))

(event EventTick
  (params (DeltaSeconds :type Float%20%28single-precision%29))
  (bind _self self)
  (if (Variables|Default|GetbSeePlayer)
    (Transformation|SetActorRotation (Math|Rotator|Lerp(Rotator) (Transformation|GetActorRotation _self) (Math|Rotator|FindLookatRotation (Transformation|GetActorLocation _self) (Transformation|GetActorLocation (Variables|Default|GetPlayer))) DeltaSeconds true)))
  (if (Variables|Default|GetAttached)
    (Transformation|SetWorldLocation (Variables|Default|GetCable) (Transformation|GetActorLocation (Variables|Default|GetPlayer)) false true)))

(event EventAction
  (if (Variables|Default|GetDrawn)
    (if (Variables|Default|GetbHasFired)
      (if (Variables|Default|GetAttached)
        (CallFunction|Grappleto)
        (elif (Variables|Default|GetbCanShoot)
          (CallFunction|ResetGrapple)
          (else
            (CallFunction|Stall))))
      (else
        (CallFunction|Fire)))
    (else
      (CallFunction|Draw))))

(fn ConstructionScript
  (Collision|SetCollisionEnabled (Variables|Default|GetSphere) "NoCollision"))

(fn FindTarget
  (bind _arrow1 (Variables|Default|GetArrow1))
  (bind _returnvalue (Transformation|GetWorldLocation _arrow1))
  (bind (_outhit _returnvalue_2) (Collision|LineTraceByChannel _returnvalue (+ _returnvalue (* (Math|Vector|GetForwardVector _arrow1) 5e+03)) "TraceTypeQuery2" false 0 "ForDuration"))
  (if _returnvalue_2
    _
    (else
      (Development|PrintString "D'ow I missed!")))
  (bind _output_get (Variables|Default|SetGrappleTarget (Math|Vector|SelectVector (.Location (Collision|BreakHitResult _outhit)) (.TraceEnd (Collision|BreakHitResult _outhit)) (.bBlockingHit (Collision|BreakHitResult _outhit)))))
  (return _output_get))