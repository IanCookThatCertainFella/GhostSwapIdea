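; BP_Enemy_Metronome is a metronome that drives the actors in its HeadBangers list on a shared tempo.
; From BeginPlay, a Beat event re-triggers itself after a delay derived from BPM.
; Each beat sends ActionMessage to every list entry implementing BPI_Beat.
; After each delay and re-trigger it also prints a debug string and plays a 2D sound.
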(event Custom|Beat
  (for _array_element (Variables|Default|GetHeadBangers)
    (if (Utilities|DoesObjectImplementInterface _array_element "/Game/GameIIIBlueprints/BPI_Beat.BPI_Beat_C")
      (Class|BPIBeat|Action(Message) _array_element)))
  (Utilities|FlowControl|Delay (/ 6e+01 (Variables|Default|GetBPM)))
  (CallFunction|Beat)
  (Development|PrintString "Beap")
  (Audio|PlaySound2D "/Game/Audio/Boomerang_A.Boomerang_A" 1.0 1.0 0.0 0 0))

(event EventBeginPlay
  (CallFunction|Beat))

(event Collision|EventActorBeginOverlap
  (params (OtherActor :type Actor%20Object%20Reference)))

(event EventTick
  (params (DeltaSeconds :type Float%20%28single-precision%29)))

(fn ConstructionScript)