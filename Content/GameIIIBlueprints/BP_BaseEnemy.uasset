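; Base enemy that turns toward a spotted player and shoots in bursts timed by beat counting.
; Pawn sensing latches the player as target, and a sphere overlap tracks whether they are in range.
; Action counts beats up to the note length, then triggers FireClip, a delayed loop of shots.
; Each shot either spawns a projectile sharing the enemy's Metronome or line-traces to damage BPI_Damagible actors.
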(event OnComponentBeginOverlap(Sphere)
  (params (OverlappedComponent :type Primitive%20Component%20Object%20Reference) (OtherActor :type Actor%20Object%20Reference) (OtherComp :type Primitive%20Component%20Object%20Reference) (OtherBodyIndex :type Integer) (bFromSweep :type Boolean) (SweepResult :type Hit%20Result%20Structure%20%28by%20ref%29))
  (if (Actor|ActorHasTag OtherActor "Player")
    (Variables|Default|SetbPlayerInRange true)))

(event OnComponentEndOverlap(Sphere)
  (params (OverlappedComponent :type Primitive%20Component%20Object%20Reference) (OtherActor :type Actor%20Object%20Reference) (OtherComp :type Primitive%20Component%20Object%20Reference) (OtherBodyIndex :type Integer))
  (if (Actor|ActorHasTag OtherActor "Player")
    (Variables|Default|SetbPlayerInRange false)))

(event OnSeePawn(PawnSensing)
  (params (Pawn :type Pawn%20Object%20Reference))
  (bind _asbp_first_person_swap (Utilities|Casting|CastToBP_FirstPersonSwap Pawn))
  (Variables|Default|SetbSeePlayer true)
  (Variables|Default|SetPlayer _asbp_first_person_swap))

(event Custom|FireClip
  (if (Math|Boolean|ANDBoolean (Variables|Default|GetbSeePlayer) (Variables|Default|GetbPlayerInRange) (not (Variables|Default|GetbIsShooting)))
    (if (Variables|Default|GetbCanShoot) :!label _label
      (Variables|Default|SetbIsShooting true)
      (CallFunction|Fire)
      (Math|Integer|IncrementInt (Variables|Default|GetShotsFired)
        (:%20%20
          (if (< (Variables|Default|GetShotsFired) (Variables|Default|GetClipCount))
            (Utilities|FlowControl|Delay (Variables|Default|GetShotDelay))
            (Development|PrintString "Bang!")
            (goto _label)
            (else
              (Variables|Default|SetbIsShooting false)
              (Variables|Default|SetbCanShoot true)
              (Variables|Default|SetShotsFired 0))))))))

(event Custom|BePossessed)

(event EventBeginPlay)

(event Collision|EventActorBeginOverlap
  (params (OtherActor :type Actor%20Object%20Reference)))

(event EventTick
  (params (DeltaSeconds :type Float%20%28single-precision%29))
  (bind _self self)
  (if (Variables|Default|GetbSeePlayer)
    (Transformation|SetActorRotation (Math|Rotator|Lerp(Rotator) (Transformation|GetActorRotation _self) (Math|Rotator|FindLookatRotation (Transformation|GetActorLocation _self) (Transformation|GetActorLocation (Variables|Default|GetPlayer))) DeltaSeconds true))))

(event EventAction
  (bind _result (Math|Integer|IncrementInt (Variables|Default|GetHeldBeats))
    (:%20%20
      (if (>= _result (Variables|Default|GetNoteLength))
        (CallFunction|FireClip)
        (Variables|Default|SetHeldBeats 0)))))

(fn ConstructionScript)

(fn Fire
  (bind _arrow1 (Variables|Default|GetArrow1))
  (bind _arrow1_2 (Variables|Default|GetArrow1))
  (bind _arrow1_3 (Variables|Default|GetArrow1))
  (bind _returnvalue (Transformation|GetWorldLocation _arrow1_2))
  (bind _returnvalue_2 (Transformation|GetWorldLocation _arrow1_3))
  (bind _returnvalue_3 (Transformation|GetWorldLocation _arrow1))
  (Audio|PlaySound2D "/Game/Audio/Boomerang_B.Boomerang_B" 1.0 1.0 0.0 0 0)
  (if (Variables|Default|GetbFireProjectile)
    (bind _outhit (Collision|LineTraceByChannel _returnvalue_2 (+ _returnvalue_2 (* (Math|Vector|GetForwardVector _arrow1_3) 5e+03)) "TraceTypeQuery1" false 0 "ForDuration"))
    (bind _returnvalue_4 (Game|SpawnActorfromClass (Variables|Default|GetProjectile) (Math|Transform|MakeTransform (+ _returnvalue_3 (* (Math|Vector|GetForwardVector (Math|Rotator|FindLookatRotation _returnvalue_3 (Math|Vector|SelectVector (.Location (Collision|BreakHitResult _outhit)) (.TraceEnd (Collision|BreakHitResult _outhit)) (.bBlockingHit (Collision|BreakHitResult _outhit))))) 1e+01)) (Math|Rotator|FindLookatRotation (+ _returnvalue_3 (* (Math|Vector|GetForwardVector (Math|Rotator|FindLookatRotation _returnvalue_3 (Math|Vector|SelectVector (.Location (Collision|BreakHitResult _outhit)) (.TraceEnd (Collision|BreakHitResult _outhit)) (.bBlockingHit (Collision|BreakHitResult _outhit))))) 1e+01)) (Math|Vector|SelectVector (.Location (Collision|BreakHitResult _outhit)) (.TraceEnd (Collision|BreakHitResult _outhit)) (.bBlockingHit (Collision|BreakHitResult _outhit))))) "Undefined" "MultiplyWithRoot" 0 0))
    (Variables|/Game/GameIIIBlueprints/BP_Projectile.BP_Projectile_C|SetMetronome _returnvalue_4 (Variables|Default|GetMetronome))
    (else
      (bind (_outhit_2 _returnvalue_5) (Collision|LineTraceByChannel _returnvalue (+ _returnvalue (* (Math|Vector|GetForwardVector _arrow1_2) 5e+03)) "TraceTypeQuery2" false 0 "ForDuration" true "(R=1.000000,G=0.000000,B=0.000000,A=1.000000)" "(R=0.000000,G=1.000000,B=0.000000,A=1.000000)" 2.0))
      (if _returnvalue_5
        (Development|PrintString (Utilities|GetDisplayName (.HitActor (Collision|BreakHitResult _outhit_2))))
        (if (Utilities|DoesObjectImplementInterface (.HitActor (Collision|BreakHitResult _outhit_2)) "/Game/GameIIIBlueprints/BPI_Damagible.BPI_Damagible_C")
          (Class|BPIDamagible|GetDamaged(Message) (.HitActor (Collision|BreakHitResult _outhit_2))))))))