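; BP_Flame is a short-lived flame actor that damages what it touches.
; On BeginPlay it waits a fixed delay of roughly half a second, then destroys itself through the Disappear event.
; While it lives, any actor entering its Capsule that implements BPI_Damagible receives GetDamagedMessage, so targets handle their own damage response.
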(event OnComponentBeginOverlap(Capsule)
  (params (OverlappedComponent :type Primitive%20Component%20Object%20Reference) (OtherActor :type Actor%20Object%20Reference) (OtherComp :type Primitive%20Component%20Object%20Reference) (OtherBodyIndex :type Integer) (bFromSweep :type Boolean) (SweepResult :type Hit%20Result%20Structure%20%28by%20ref%29))
  (if (Utilities|DoesObjectImplementInterface OtherActor "/Game/GameIIIBlueprints/BPI_Damagible.BPI_Damagible_C")
    (Class|BPIDamagible|GetDamaged(Message) OtherActor)))

(event Custom|Disappear
  (Actor|DestroyActor))

(event EventBeginPlay
  (Utilities|FlowControl|Delay (Utilities|Operators|Divide 1e+02 6e+01 3.0))
  (CallFunction|Disappear))

(event Collision|EventActorBeginOverlap
  (params (OtherActor :type Actor%20Object%20Reference)))

(event EventTick
  (params (DeltaSeconds :type Float%20%28single-precision%29)))

(fn ConstructionScript
  (|CallParentFunction))